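; Phase 2 robot boss that damages pawns overlapping its Box and gets stunned when the Box overlaps a non-pawn actor.
; Stun is written to the AI controller's blackboard as IsStunned, behind a DoOnce gate.
; ResetStunTimer clears the key and reopens the gate, but the timer node that would schedule it after StunDuration is unconnected.
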(event OnComponentBeginOverlap(Box)
  (params (OverlappedComponent :type Primitive%20Component%20Object%20Reference) (OtherActor :type Actor%20Object%20Reference) (OtherComp :type Primitive%20Component%20Object%20Reference) (OtherBodyIndex :type Integer) (bFromSweep :type Boolean) (SweepResult :type Hit%20Result%20Structure%20%28by%20ref%29))
  (if (!= OtherActor self)
    (bind _aspawn (Utilities|Casting|CastToPawn OtherActor)
      (:then
        (bind _returnvalue (Game|Damage|ApplyDamage _aspawn (Variables|Default|GetDamagePerHit) (Pawn|GetController) _aspawn "/Script/Engine.DamageType"))
        (Development|PrintString (Utilities|String|Append "Damage given :" (Utilities|String|ToString(Float) _returnvalue)) true true "(R=1.000000,G=0.021345,B=0.000000,A=1.000000)" 3.0))
      (:CastFailed
        (Utilities|FlowControl|DoOnce false
          (:Completed
            (CallFunction|SendStunEvent)
            (Development|PrintString "should be stun ")))))))

(event Custom|SendStunEvent
  (bind _returnvalue (Utilities|GetAIBlackboard))
  (AI|Components|Blackboard|SetValueasBool _returnvalue (Utilities|Name|MakeLiteralName "IsStunned") true))

(event Custom|ResetStunTimer
  (bind _returnvalue (Utilities|GetAIBlackboard))
  (AI|Components|Blackboard|SetValueasBool _returnvalue (Utilities|Name|MakeLiteralName "IsStunned") false)
  (Development|PrintString "stun reset" true true "(R=1.000000,G=0.021645,B=0.000000,A=1.000000)" 5.0)
  (CallFunction|ResetStun))

(event Custom|ResetStun
  (Development|PrintString "reset stun effect" true true "(R=0.000000,G=1.000000,B=0.034366,A=1.000000)" 5.0)
  (Utilities|FlowControl|DoOnce false) ; enters at Reset
)

(fn ConstructionScript)